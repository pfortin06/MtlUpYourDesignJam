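; Box actor that tracks whether it can be pushed, based on overlaps with other actors.
; Its Box component's begin-overlap event confirms the overlap and sets the CanPush flag, while the actor's end-overlap event clears it for any departing actor.
; Both events print debug strings; no push movement is implemented here.
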(event OnComponentBeginOverlap(Box)
  (params (OverlappedComponent :type Primitive%20Component%20Object%20Reference) (OtherActor :type Actor%20Object%20Reference) (OtherComp :type Primitive%20Component%20Object%20Reference) (OtherBodyIndex :type Integer) (bFromSweep :type Boolean) (SweepResult :type Hit%20Result%20Structure%20%28by%20ref%29))
  (if (Collision|IsOverlappingActor (Variables|Default|GetBox) OtherActor :!class /Script/Engine.PrimitiveComponent)
    (bind _output_get (Variables|Default|SetcanPush true))
    (Development|PrintString (Utilities|String|ToString(Boolean) _output_get))
    (else
      (Development|PrintString "false"))))

(event EventBeginPlay)

(event Collision|EventActorBeginOverlap
  (params (OtherActor :type Actor%20Object%20Reference)))

(event EventTick
  (params (DeltaSeconds :type Float%20%28single-precision%29)))

(event Collision|EventActorEndOverlap
  (params (OtherActor :type Actor%20Object%20Reference))
  (bind _output_get (Variables|Default|SetcanPush false))
  (Development|PrintString (Utilities|String|ToString(Boolean) _output_get)))

(fn ConstructionScript)